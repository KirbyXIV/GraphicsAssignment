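; BP_Enemy is an enemy pawn that wanders the navmesh and chases pawns it sees.
; It loops AIMoveTo to random nearby navigable points, pausing briefly after each success.
; PawnSensing sightings raise walk speed once through a DoOnce and move it toward the seen pawn.
; Each sighting restarts a RetriggerableDelay, which on expiry slows the enemy, resets the DoOnce and resumes wandering.
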(event OnSeePawn(PawnSensing)
  (params (Pawn :type Pawn%20Object%20Reference))
  (Utilities|FlowControl|Sequence
    (:then_0
      (Utilities|FlowControl|DoOnce false
        (:Completed
          (Variables|/Script/Engine.CharacterMovementComponent|SetMaxWalkSpeed (Variables|Character|GetCharacterMovement) 5e+02))))
    (:then_1
      (AI|AIMoveTo self "0, 0, 0" Pawn 5.0 false
        (:then
          (Utilities|FlowControl|RetriggerableDelay 2.0)
          (Variables|/Script/Engine.CharacterMovementComponent|SetMaxWalkSpeed (Variables|Character|GetCharacterMovement) 1.3e+02)
          (CallFunction|CanSprintAgain)
          (CallFunction|MovetoRandomLoc))))))

(event Custom|MoveToRandomLoc
  (bind _randomlocation (Class|NavigationSystemV1|GetRandomLocationinNavigableRadius (Transformation|GetActorLocation) 4e+03 0 0))
  (AI|AIMoveTo self _randomlocation 0 2e+01 false
    (:OnSuccess
      (Utilities|FlowControl|Delay 2.0)
      (CallFunction|MovetoRandomLoc))))

(event Custom|CanSprintAgain
  (Utilities|FlowControl|DoOnce false) ; enters at Reset
)

(event EventBeginPlay
  (CallFunction|MovetoRandomLoc))

(fn ConstructionScript)