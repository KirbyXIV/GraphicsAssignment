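; BP_Door is a door actor that opens or closes according to the state of a set of plates.
; Its plate event checks every entry in Plates, playing a timeline from the start if all are active and reversing it otherwise.
; The timeline animates the door by scaling its height with fixed width and depth, rather than moving it.
; StartsOpen collapses the actor to zero scale on BeginPlay.
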(event Custom|onPlateActive_Event
  (Variables|Default|SetplateActive true)
  (for _array_element (Variables|Default|GetPlates)
    (if (not (Variables|/Game/MyBlueprints/BP_PressurePlate.BP_PressurePlate_C|GetisActive _array_element))
      (Variables|Default|SetplateActive false)))
  (if (Variables|Default|GetplateActive)
    (bind _dooropening (Timeline|Timeline PlayFromStart)
      (:Update
        (Transformation|SetActorScale3D (Math|Vector|MakeVector 1.75 1.5 (* _dooropening 2.5)))))
    (else
      (Timeline|Timeline Reverse))))

(event EventBeginPlay
  (if (Variables|Default|GetstartsOpen)
    (Transformation|SetActorScale3D "0, 0, 0")))

(fn ConstructionScript)