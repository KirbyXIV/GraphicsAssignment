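; Pressure plate that sinks when a BP_ThirdPersonCharacter steps on it and rises again when the character leaves.
; Box begin and end overlaps each play their own timeline from the start, lerping the relative Z of Sphere1 down or back up.
; The plate only animates and signals no other actor.
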(event OnComponentBeginOverlap(Box)
  (params (OverlappedComponent :type Primitive%20Component%20Object%20Reference) (OtherActor :type Actor%20Object%20Reference) (OtherComp :type Primitive%20Component%20Object%20Reference) (OtherBodyIndex :type Integer) (bFromSweep :type Boolean) (SweepResult :type Hit%20Result%20Structure%20%28by%20ref%29))
  (Utilities|Casting|CastToBP_ThirdPersonCharacter OtherActor)
  (bind _plate_go_down (Timeline|Timeline PlayFromStart)
    (:Update
      (Transformation|SetRelativeLocation (Variables|Default|GetSphere1) (Math|Vector|MakeVector 0.0 0.0 (Math|Float|Lerp 1e+01 0.0 _plate_go_down)) false false))))

(event OnComponentEndOverlap(Box)
  (params (OverlappedComponent :type Primitive%20Component%20Object%20Reference) (OtherActor :type Actor%20Object%20Reference) (OtherComp :type Primitive%20Component%20Object%20Reference) (OtherBodyIndex :type Integer))
  (Utilities|Casting|CastToBP_ThirdPersonCharacter OtherActor)
  (bind _plate_go_down (Timeline|Timeline_0 PlayFromStart)
    (:Update
      (Transformation|SetRelativeLocation (Variables|Default|GetSphere1) (Math|Vector|MakeVector 0.0 0.0 (Math|Float|Lerp 0.0 1e+01 _plate_go_down)) false false))))

(fn ConstructionScript)